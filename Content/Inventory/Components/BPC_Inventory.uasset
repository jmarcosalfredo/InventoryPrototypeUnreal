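; Player inventory component that handles item pickup, money and health, and creates their inventory, interact and health bar widgets.
; A per-tick forward sphere trace toggles the interact prompt, and the interact input reuses it to collect BP_Item actors.
; Items go into fixed-size arrays per type, stacking up to DT_Item limits before taking empty slots.
; Capsule overlap collects money valued through DT_Money, while N and M keys adjust health.
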(event `self.ReceiveTick`
  (params (DeltaSeconds :type "Float (single-precision)"))
  (bind _wbp_interact (`self.WBP_Interact`))
  (bind (_item _founditem) (`self.TraceItemToPickUp`))
  (set `/Game/Inventory/Widgets/WPB_ItemInfo.Item` _item (`/Game/Inventory/Widgets/WBP_Interact.WPB_ItemInfo` (`self.WBP_Interact`)))
  (if _founditem
    (`UserWidget.AddToViewport` _wbp_interact 0)
    (else
      (`Widget.RemoveFromParent` _wbp_interact))))

(event `self.ReceiveBeginPlay`
  (bind (_swords _shields _eatables) (break `/Game/Inventory/Structs/S_AllItems` (`self.AllItems`)))
  (`EnhancedInputSubsystemInterface.AddMappingContext` (pcsubsystem `EnhancedInputLocalPlayerSubsystem` (`GameplayStatics.GetPlayerController` 0)) "/Game/Inventory/Inputs/IMC_Inventory.IMC_Inventory" 0 (struct))
  (bind _returnvalue (`|CreateWidget` "/Game/Inventory/Widgets/WBP_Inventory.WBP_Inventory_C"))
  (set `self.WBP_Inventory` _returnvalue)
  (bind _asbp_third_person_character (cast `/Game/ThirdPerson/Blueprints/BP_ThirdPersonCharacter` (`GameplayStatics.GetPlayerCharacter` 0)))
  (bind _output_get (set `self.As BP Third Person Character` _asbp_third_person_character))
  (add `PrimitiveComponent.OnComponentBeginOverlap` (`Character.CapsuleComponent` _output_get) (`|CreateDelegate` :!event `PickUpMoney`))
  (`self.HealthBarInit`)
  (bind _returnvalue_2 (`|CreateWidget` "/Game/Inventory/Widgets/WBP_Interact.WBP_Interact_C"))
  (set `self.WBP_Interact` _returnvalue_2)
  (`KismetArrayLibrary.Array_Resize` _swords 5)
  (`KismetArrayLibrary.Array_Resize` _shields 8)
  (`KismetArrayLibrary.Array_Resize` _eatables 20)
  (`/Game/Inventory/Widgets/WBP_Inventory.UpdateItemsInInventoryUI` (`self.WBP_Inventory`) (`self.AllItems`)))

(event `Key|N`
  (params (Key :type "Key Structure"))
  (:`Pressed`
    (`self.IncreaseHealth` 0.5)))

(event `Key|M`
  (params (Key :type "Key Structure"))
  (:`Pressed`
    (`self.DecreaseHealth` 0.5)))

(event `EnhancedInput|/Game/Inventory/Inputs/IA_Inventory`
  (params (ActionValue :type Boolean) (ElapsedSeconds :type "Float (double-precision)") (TriggeredSeconds :type "Float (double-precision)") (InputAction :type "InputAction Object Reference" :default "/Game/Inventory/Inputs/IA_Inventory.IA_Inventory"))
  (bind _returnvalue (`GameplayStatics.GetPlayerController` 0))
  (:`Triggered`
    (`UserWidget.AddToViewport` (`self.WBP_Inventory`) 0)
    (set `PlayerController.bShowMouseCursor` false _returnvalue)
    (`WidgetBlueprintLibrary.SetInputMode_UIOnlyEx` _returnvalue (`self.WBP_Inventory`))))

(event `EnhancedInput|/Game/Inventory/Inputs/IA_Interact`
  (params (ActionValue :type Boolean) (ElapsedSeconds :type "Float (double-precision)") (TriggeredSeconds :type "Float (double-precision)") (InputAction :type "InputAction Object Reference" :default "/Game/Inventory/Inputs/IA_Interact.IA_Interact"))
  (:`Triggered`
    (bind (_item _founditem _itemactor) (`self.TraceItemToPickUp`))
    (if _founditem
      (bind _success (`self.AddToInventory` _item))
      (if _success
        (`Actor.K2_DestroyActor` _itemactor)
        (`/Game/Inventory/Widgets/WBP_Inventory.UpdateItemsInInventoryUI` (`self.WBP_Inventory`) (`self.AllItems`))))))

(fn `AddToInventory`
  (params (Item :type "/Game/Inventory/Structs/S_Slot Structure"))
  (returns (Success :type Boolean))
  (bind (_itemid _quantity _itemtype) (break `/Game/Inventory/Structs/S_Slot` (`local.Item`)))
  (bind (_itemid_2 _quantity_2 _itemtype_2) (break `/Game/Inventory/Structs/S_Slot` (`local.Item`)))
  (bind (_itemid_3 _quantity_3 _itemtype_3) (break `/Game/Inventory/Structs/S_Slot` (`local.Item`)))
  (bind (_itemid_4 _quantity_4) (break `/Game/Inventory/Structs/S_Slot` (`local.Item`)))
  (switch `/Game/Inventory/Enums/E_ItemType` (`.ItemType_9_8098EAD84F2F0DBF4FAB1EA1FDCD5C6A` (break `/Game/Inventory/Structs/S_Slot` Item))
    (:`NewEnumerator0`
      (for (_array_element _array_index) (`.Swords_3_9206C7874C0F04401BB425A56AE23205` (break `/Game/Inventory/Structs/S_AllItems` (`self.AllItems`)))
        (bind (_itemid_5 _quantity_5) (break `/Game/Inventory/Structs/S_Slot` _array_element))
        (if (== (`.RowName` (break `DataTableRowHandle` _itemid_5)) (`.RowName` (break `DataTableRowHandle` (`.ItemID_3_319CEC14412D7758CB1068BDF4262136` (break `/Game/Inventory/Structs/S_Slot` (`local.Item`))))))
          (bind _returnvalue (`|GetDataTableRow` "/Game/Inventory/DataTables/DT_Item.DT_Item" (`.RowName` (break `DataTableRowHandle` (`.ItemID_3_319CEC14412D7758CB1068BDF4262136` (break `/Game/Inventory/Structs/S_Slot` (`local.Item`))))))
            (:`then`
              (bind _returnvalue_2 (+ (`.Quantity_6_C7691B384930BEFBC73DE7A542B4094D` (break `/Game/Inventory/Structs/S_Slot` (`local.Item`))) _quantity_5))
              (if (>= (`.StackSize_10_D8251B334EC53E9B5C6DC184A9C58895` (break `/Game/Inventory/Structs/S_Item` _returnvalue)) _returnvalue_2)
                (`KismetArrayLibrary.Array_Set` (`.Swords_3_9206C7874C0F04401BB425A56AE23205` (break `/Game/Inventory/Structs/S_AllItems` (`self.AllItems`))) _array_index (make `/Game/Inventory/Structs/S_Slot` _itemid_3 _returnvalue_2 _itemtype_3))
                (return true))))))
      (for (_array_element_2 _array_index_2) (`.Swords_3_9206C7874C0F04401BB425A56AE23205` (break `/Game/Inventory/Structs/S_AllItems` (`self.AllItems`)))
        (if (== (`.Quantity_6_C7691B384930BEFBC73DE7A542B4094D` (break `/Game/Inventory/Structs/S_Slot` _array_element_2)) 0)
          (`KismetArrayLibrary.Array_Set` (`.Swords_3_9206C7874C0F04401BB425A56AE23205` (break `/Game/Inventory/Structs/S_AllItems` (`self.AllItems`))) _array_index_2 (`local.Item`))
          (return true)))
      (return false))
    (:`NewEnumerator1`
      (for (_array_element_3 _array_index_3) (`.Shields_5_E46003EC4C977DDABFBEE9A1D7491B44` (break `/Game/Inventory/Structs/S_AllItems` (`self.AllItems`)))
        (bind (_itemid_6 _quantity_6) (break `/Game/Inventory/Structs/S_Slot` _array_element_3))
        (if (== (`.RowName` (break `DataTableRowHandle` _itemid_6)) (`.RowName` (break `DataTableRowHandle` (`.ItemID_3_319CEC14412D7758CB1068BDF4262136` (break `/Game/Inventory/Structs/S_Slot` (`local.Item`))))))
          (bind _returnvalue_3 (`|GetDataTableRow` "/Game/Inventory/DataTables/DT_Item.DT_Item" (`.RowName` (break `DataTableRowHandle` (`.ItemID_3_319CEC14412D7758CB1068BDF4262136` (break `/Game/Inventory/Structs/S_Slot` (`local.Item`))))))
            (:`then`
              (bind _returnvalue_4 (+ (`.Quantity_6_C7691B384930BEFBC73DE7A542B4094D` (break `/Game/Inventory/Structs/S_Slot` (`local.Item`))) _quantity_6))
              (if (>= (`.StackSize_10_D8251B334EC53E9B5C6DC184A9C58895` (break `/Game/Inventory/Structs/S_Item` _returnvalue_3)) _returnvalue_4)
                (`KismetArrayLibrary.Array_Set` (`.Shields_5_E46003EC4C977DDABFBEE9A1D7491B44` (break `/Game/Inventory/Structs/S_AllItems` (`self.AllItems`))) _array_index_3 (make `/Game/Inventory/Structs/S_Slot` _itemid_2 _returnvalue_4 _itemtype_2))
                (return true))))))
      (for (_array_element_4 _array_index_4) (`.Shields_5_E46003EC4C977DDABFBEE9A1D7491B44` (break `/Game/Inventory/Structs/S_AllItems` (`self.AllItems`)))
        (if (== (`.Quantity_6_C7691B384930BEFBC73DE7A542B4094D` (break `/Game/Inventory/Structs/S_Slot` _array_element_4)) 0)
          (`KismetArrayLibrary.Array_Set` (`.Shields_5_E46003EC4C977DDABFBEE9A1D7491B44` (break `/Game/Inventory/Structs/S_AllItems` (`self.AllItems`))) _array_index_4 (`local.Item`))
          (return true)))
      (return false))
    (:`NewEnumerator2`
      (for (_array_element_5 _array_index_5) (`.Eatables_7_E88DA8DB4E12A52267C95689589683D6` (break `/Game/Inventory/Structs/S_AllItems` (`self.AllItems`)))
        (bind (_itemid_7 _quantity_7) (break `/Game/Inventory/Structs/S_Slot` _array_element_5))
        (if (== (`.RowName` (break `DataTableRowHandle` _itemid_7)) (`.RowName` (break `DataTableRowHandle` (`.ItemID_3_319CEC14412D7758CB1068BDF4262136` (break `/Game/Inventory/Structs/S_Slot` (`local.Item`))))))
          (bind _returnvalue_5 (`|GetDataTableRow` "/Game/Inventory/DataTables/DT_Item.DT_Item" (`.RowName` (break `DataTableRowHandle` _itemid_4)))
            (:`then`
              (bind _returnvalue_6 (+ _quantity_4 _quantity_7))
              (if (>= (`.StackSize_10_D8251B334EC53E9B5C6DC184A9C58895` (break `/Game/Inventory/Structs/S_Item` _returnvalue_5)) _returnvalue_6)
                (`KismetArrayLibrary.Array_Set` (`.Eatables_7_E88DA8DB4E12A52267C95689589683D6` (break `/Game/Inventory/Structs/S_AllItems` (`self.AllItems`))) _array_index_5 (make `/Game/Inventory/Structs/S_Slot` _itemid _returnvalue_6 _itemtype))
                (return true))))))
      (for (_array_element_6 _array_index_6) (`.Eatables_7_E88DA8DB4E12A52267C95689589683D6` (break `/Game/Inventory/Structs/S_AllItems` (`self.AllItems`)))
        (if (== (`.Quantity_6_C7691B384930BEFBC73DE7A542B4094D` (break `/Game/Inventory/Structs/S_Slot` _array_element_6)) 0)
          (`KismetArrayLibrary.Array_Set` (`.Eatables_7_E88DA8DB4E12A52267C95689589683D6` (break `/Game/Inventory/Structs/S_AllItems` (`self.AllItems`))) _array_index_6 (`local.Item`))
          (return true)))
      (return false))))

(fn `DecreaseHealth`
  (params (HealthToRemove :type "Float (double-precision)"))
  (set `self.Health` (- (`self.Health`) HealthToRemove))
  (`/Game/Inventory/Widgets/WBP_HealthBar.UpdateHealthBar` (`self.WPB_HealthBar`)))

(fn `HealthBarInit`
  (bind _returnvalue (`|CreateWidget` "/Game/Inventory/Widgets/WBP_HealthBar.WBP_HealthBar_C"))
  (bind _output_get (set `self.WPB_HealthBar` _returnvalue))
  (`UserWidget.SetPositionInViewport` _output_get (5.0 5.0) true)
  (`UserWidget.AddToViewport` _output_get 0))

(fn `IncreaseHealth`
  (params (HealthToAdd :type "Float (double-precision)"))
  (set `self.Health` (+ HealthToAdd (`self.Health`)))
  (`/Game/Inventory/Widgets/WBP_HealthBar.UpdateHealthBar` (`self.WPB_HealthBar`)))

(fn `PickUpMoney`
  (params (OverlappedComponent :type "PrimitiveComponent Object Reference") (OtherActor :type "Actor Object Reference") (OtherComp :type "PrimitiveComponent Object Reference") (OtherBodyIndex :type Integer) (bFromSweep :type Boolean) (SweepResult :type "HitResult Structure (by ref)"))
  (bind _asbp_money (cast `/Game/Inventory/Blueprints/BP_Money` OtherActor))
  (bind (_moneytype_datatable _moneytype_rowname) (break `DataTableRowHandle` (`/Game/Inventory/Blueprints/BP_Money.MoneyType` _asbp_money)))
  (bind _returnvalue (`|GetDataTableRow` "/Game/Inventory/DataTables/DT_Money.DT_Money" _moneytype_rowname)
    (:`then`
      (set `self.MoneyAmountComponent` (+ (`.Amount_5_282D3B6E4392463C9647D992F54FAA9A` (break `/Game/Inventory/Structs/S_Money` _returnvalue)) (`self.MoneyAmountComponent`)))
      (`Actor.K2_DestroyActor` _asbp_money)
      (set `/Game/Inventory/Widgets/WBP_Inventory.MoneyAmountWidget` (`self.MoneyAmountComponent`) (`self.WBP_Inventory`))
      (return))))

(fn `TraceItemToPickUp`
  (returns (Item :type "/Game/Inventory/Structs/S_Slot Structure") (FoundItem :type Boolean) (ItemActor :type "Actor Object Reference"))
  (bind _returnvalue (`GameplayStatics.GetPlayerCharacter` 0))
  (bind _returnvalue_2 (- (`Actor.K2_GetActorLocation` _returnvalue) (0.0 0.0 60.0)))
  (bind _outhit (`KismetSystemLibrary.SphereTraceSingle` :`Start` _returnvalue_2 :`End` (+ _returnvalue_2 (* (`Actor.GetActorForwardVector` _returnvalue) 100.0)) :`Radius` 30.0 :`TraceChannel` "TraceTypeQuery1" :`DrawDebugType` "ForOneFrame"))
  (bind _asbp_item (cast `/Game/Inventory/Blueprints/BP_Item` (`.HitActor` (`GameplayStatics.BreakHitResult` _outhit)))
    (:`then`
      (return (`/Game/Inventory/Blueprints/BP_Item.Item` _asbp_item) true (`.HitActor` (`GameplayStatics.BreakHitResult` _outhit))))
    (:`CastFailed`
      (return (struct) false null))))